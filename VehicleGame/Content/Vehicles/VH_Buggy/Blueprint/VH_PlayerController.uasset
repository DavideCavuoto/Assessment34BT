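; Player controller for the buggy vehicle that tracks checkpoint progress and the race finish.
; Overlap updates show the checkpoint HUD and flag three checkpoints by display name.
; Reaching the FinishLine trigger box with all three flags set disables the buggy's input.
; Lap counting, best-time tracking from game state time and the lap-completed HUD update are present but disconnected, so the race ends after one pass.
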(event `Event VH OverlapUpdate (Controller)`
  (params (Actor :type "Actor Object Reference"))
  ;[1 1 1] Lap Tracking setup
  (bind _asvehicle_track_point (cast `VehicleTrackPoint` Actor)
    (:`then`
      (bind _asvh_hud (cast `/Game/Vehicles/VH_Buggy/Blueprint/VH_HUD` (`self.GetHUD`)))
      (`/Game/Vehicles/VH_Buggy/Blueprint/VH_HUD.Event DisplayCheckpoint (HUD)` _asvh_hud)
      (bind _returnvalue (`KismetSystemLibrary.GetDisplayName` _asvehicle_track_point))
      (if (`KismetStringLibrary.EqualEqual_StrStr` _returnvalue "CheckPointA")
        (set `self.PointA` true)
        (elif (`KismetStringLibrary.EqualEqual_StrStr` _returnvalue "CheckPointB")
          (set `self.PointB` true)
          (elif (`KismetStringLibrary.EqualEqual_StrStr` _returnvalue "CheckPointC")
            (set `self.PointC` true)))))
    (:`CastFailed`
      (bind _astrigger_box (cast `TriggerBox` Actor))
      (if (`KismetStringLibrary.EqualEqual_StrStr` (`KismetSystemLibrary.GetDisplayName` _astrigger_box) "FinishLine")
        (if (`self.PointA`)
          (if (`self.PointB`)
            (if (`self.PointC`)
              ;[0.288 1 0.2604] Disable Inputs After Finishing the Race
              (bind _asvh_buggy (cast `/Game/Vehicles/VH_Buggy/Blueprint/VH_Buggy` (`GameplayStatics.GetPlayerPawn` 0)))
              (`/Game/Vehicles/VH_Buggy/Blueprint/VH_Buggy.DisableInputAfterFinish` _asvh_buggy))))))))

(fn `UserConstructionScript`)