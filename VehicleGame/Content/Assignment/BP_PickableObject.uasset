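; BP_PickableObject is a spinning collectible that a VH_Buggy picks up to earn points, with a rare variant flagged by IsRare.
; The construction script gives rare objects a different material, and Tick rotates the Cube while resetting actor rotation to zero.
; On Sphere overlap with the buggy, an IsPickedUp guard allows one pickup, which passes IsRare to MyGameInstance.IncrementPoints and hides the Cube rather than destroying the actor.
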(event `self.ReceiveBeginPlay`)

(event `self.ReceiveTick`
  (params (DeltaSeconds :type "Float (single-precision)"))
  ;[1 1 1] Pickable Object Rotation
  (`SceneComponent.K2_AddRelativeRotation` (`self.Cube`) (struct :`Yaw` 1.0) false false)
  (`self.K2_SetActorRelativeRotation` (struct)))

(event `self.Sphere.OnComponentBeginOverlap`
  (params (OverlappedComponent :type "PrimitiveComponent Object Reference") (OtherActor :type "Actor Object Reference") (OtherComp :type "PrimitiveComponent Object Reference") (OtherBodyIndex :type Integer) (bFromSweep :type Boolean) (SweepResult :type "HitResult Structure (by ref)"))
  ;[1 1 1] Pickable Object Flow
  (cast `/Game/Vehicles/VH_Buggy/Blueprint/VH_Buggy` OtherActor)
  (if (not (`self.IsPickedUp`))
    (`|ExecutionSequence`
      (:`then_0`
        (bind _asmy_game_instance (cast `/Game/Assignment/MyGameInstance` (`GameplayStatics.GetGameInstance`)))
        (`/Game/Assignment/MyGameInstance.IncrementPoints` _asmy_game_instance (`self.IsRare`)))
      (:`then_1`
        (set `self.IsPickedUp` true))
      (:`then_2`
        (`self.DeactivateOnPickUp`)))))

(fn `DeactivateOnPickUp`
  (if (`self.IsPickedUp`)
    (`SceneComponent.SetHiddenInGame` (`self.Cube`) true true)))

(fn `UserConstructionScript`
  (if (`self.IsRare`)
    (`PrimitiveComponent.SetMaterial` (`self.Cube`) 0 "/Game/Assignment/M_RarePickableObject.M_RarePickableObject")))